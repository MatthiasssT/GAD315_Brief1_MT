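; BP_Button1 is a proximity button that restarts one or two selected Niagara particle effects when interacted with.
; Sphere overlaps with the player character toggle an in-range flag, which shows or hides the widget.
; While in range, the button stores itself in the character's BpButtonRef.
; CallInteract fires Trigger only while in range, resetting the first system and the optional second one.
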(event `self.ReceiveBeginPlay`
  (bind _asbp_third_person_character (cast `/Game/_Main/_Blueprints/BP_ThirdPersonCharacter` (`GameplayStatics.GetPlayerCharacter` 0)))
  (set `self.As BP Third Person Character` _asbp_third_person_character)
  (`self.InRange?`))

(event `self.Sphere.OnComponentBeginOverlap`
  (params (OverlappedComponent :type "PrimitiveComponent Object Reference") (OtherActor :type "Actor Object Reference") (OtherComp :type "PrimitiveComponent Object Reference") (OtherBodyIndex :type Integer) (bFromSweep :type Boolean) (SweepResult :type "HitResult Structure (by ref)"))
  (if (== OtherActor (`self.As BP Third Person Character`))
    (set `self.PlayerInRange?` true)
    (`self.InRange?`)))

(event `self.Sphere.OnComponentEndOverlap`
  (params (OverlappedComponent :type "PrimitiveComponent Object Reference") (OtherActor :type "Actor Object Reference") (OtherComp :type "PrimitiveComponent Object Reference") (OtherBodyIndex :type Integer))
  (if (== OtherActor (`self.As BP Third Person Character`))
    (set `self.PlayerInRange?` false)
    (`self.InRange?`)))

(event `InRange?`
  (bind _widget (`self.Widget`))
  (if (`self.PlayerInRange?`)
    (`SceneComponent.SetVisibility` _widget true false)
    (set `/Game/_Main/_Blueprints/BP_ThirdPersonCharacter.BpButtonRef` self (`self.As BP Third Person Character`))
    (else
      (`SceneComponent.SetVisibility` _widget false false))))

(event `/Game/_Main/_Blueprints/BPI_Interactable1.CallInteract`
  (if (`self.PlayerInRange?`)
    (`self.Trigger`)))

(event `Trigger`
  (`NiagaraComponent.ResetSystem` (`NiagaraActor.NiagaraComponent` (`self.Selected Particle System`)))
  (bind _selected_particle_system2 (`self.Selected Particle System2`)
    (:`then`
      (`NiagaraComponent.ResetSystem` (`NiagaraActor.NiagaraComponent` _selected_particle_system2)))
    (:`else`)))

(fn `UserConstructionScript`)